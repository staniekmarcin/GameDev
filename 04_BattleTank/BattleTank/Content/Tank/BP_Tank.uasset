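; BP_Tank is the tank pawn, routing track, aiming and fire input to its components.
; TankMovement drives the two tracks, which also take direct throttle input, while TankAiming handles the turret, barrel and firing.
; Aim axes rotate the AzimuthGimbal and SpringArm separately from the turret.
; BeginPlay reapplies meshes and physical materials as a compile-reset workaround, initialises both components and links the health bar widget to the tank.
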(event `self.ReceiveBeginPlay`
  ;[1 1 1] Temporary fix for turret and barrel static mesh reset after compile
  (`StaticMeshComponent.SetStaticMesh` (`self.Turret`) "/Game/Tank/tank_fbx_Turret_turret_001.tank_fbx_Turret_turret_001")
  (`StaticMeshComponent.SetStaticMesh` (`self.Barrel`) "/Game/Tank/tank_fbx_Barrel.tank_fbx_Barrel")
  (`StaticMeshComponent.SetStaticMesh` (`self.LeftTrack`) "/Game/Tank/tank_fbx_Track_track_001.tank_fbx_Track_track_001")
  (`StaticMeshComponent.SetStaticMesh` (`self.RightTrack`) "/Game/Tank/tank_fbx_Track_track_001.tank_fbx_Track_track_001")
  ;[1 1 1] Temporary fix phycis material reset after compile
  (`PrimitiveComponent.SetPhysMaterialOverride` (`self.RightTrack`) "/Game/Tank/Track.Track")
  (`PrimitiveComponent.SetPhysMaterialOverride` (`self.LeftTrack`) "/Game/Tank/Track.Track")
  (`TankMovementComponent.Initialise` (`self.TankMovement`) (`self.LeftTrack`) (`self.RightTrack`))
  (`TankAimingComponent.Initialise` (`self.TankAiming`) (`self.Barrel`) (`self.Turret`))
  (`self.InitialiseHealthBarWidget`))

(event `self.ReceiveTick`
  (params (DeltaSeconds :type "Float (single-precision)"))
  ;[1 1 1] Console Print for Health
)

(event `InputAxis|AimAzimuth`
  (params (AxisValue :type "Float (single-precision)"))
  ;[1 1 1] Balistics Input Biding
  (`SceneComponent.K2_AddLocalRotation` (`self.AzimuthGimbal`) (`KismetMathLibrary.MakeRotator` 0.0 0.0 AxisValue) false false))

(event `InputAxis|LeftTrackThrottle`
  (params (AxisValue :type "Float (single-precision)"))
  ;[1 1 1] Movement Input Binding
  (`TankTrack.SetThrottle` (`self.LeftTrack`) AxisValue))

(event `InputAxis|RightTrackThrottle`
  (params (AxisValue :type "Float (single-precision)"))
  ;[1 1 1] Movement Input Binding
  (`TankTrack.SetThrottle` (`self.RightTrack`) AxisValue))

(event `InputAxis|AimElevation`
  (params (AxisValue :type "Float (single-precision)"))
  ;[1 1 1] Balistics Input Biding
  (`SceneComponent.K2_AddLocalRotation` (`self.SpringArm`) (`KismetMathLibrary.MakeRotator` 0.0 AxisValue) false false))

(event `InputAxis|MoveForward`
  (params (AxisValue :type "Float (single-precision)"))
  ;[1 1 1] Movement Input Binding
  (`TankMovementComponent.IntendMoveForward` (`self.TankMovement`) AxisValue))

(event `InputAction|Fire`
  (params (Key :type "Key Structure"))
  ;[1 1 1] Balistics Input Biding
  (:`Pressed`
    (`TankAimingComponent.Fire` (`self.TankAiming`))))

(event `InputAxis|TurnRight`
  (params (AxisValue :type "Float (single-precision)"))
  ;[1 1 1] Movement Input Binding
  (`TankMovementComponent.IntendTurnRight` (`self.TankMovement`) AxisValue))

(fn `InitialiseHealthBarWidget`
  (bind _asbp_health_bar (cast `/Game/UI/BP_HealthBar` (`WidgetComponent.GetUserWidgetObject` (`self.HealthBar`))))
  (set `/Game/UI/BP_HealthBar.MyTank` self _asbp_health_bar)
  (return))

(fn `UserConstructionScript`)